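; Actor component that gives its owner a Braid-style time rewind, toggled through UpdateTimeReverse.
; While time runs forward, Tick records transform and static mesh linear and angular velocities into TimeFrames.
; A ten-second rolling cap exists, but Tick passes zero delta time, so it never trims.
; While reversing, it restores frames from the newest backwards, skipping by ReverseSpeed and deleting consumed frames until the history runs out.
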(event `/Game/Blueprints/BI_Time.UpdateTimeReverse`
  (params (IsTimeReversing :type Boolean))
  (set `self.IsTimeReversing` IsTimeReversing))

(event `self.ReceiveBeginPlay`
  (if (not (`self.IsInited`))
    (set `self.IsInited` true)
    (set `self.Owner` (`self.GetOwner`))))

(event `self.ReceiveTick`
  (params (DeltaSeconds :type "Float (single-precision)"))
  (if (`self.IsInited`)
    (if (`self.IsTimeReversing`)
      (if (not (`self.IsOutData`))
        (`self.ExcuTimeinfo`))
      (else
        (`self.RecordTimeinfo` 0.0)))))

(fn `ExcuTimeinfo`
  (bind _timeframes (`self.TimeFrames`))
  (bind _timeframes_2 (`self.TimeFrames`))
  (bind _returnvalue (- (`KismetArrayLibrary.Array_LastIndex` _timeframes) (`self.ReverseSpeed`)))
  (if (<= (`KismetArrayLibrary.Array_Length` (`self.TimeFrames`)) 0)
    (set `self.RecordTimeLength` 0.0)
    (set `self.IsOutData` true)
    (elif (>= _returnvalue 0)
      (`self.SetActorInfo` _timeframes _returnvalue)
      (for _index (range (+ (`self.ReverseSpeed`) 1))
        (bind _returnvalue_2 (- (`KismetArrayLibrary.Array_LastIndex` _timeframes_2) _index))
        (bind (_output_location _output_rotation _output_linearvelocity _output_angularvelocity _output_deltatime) (break `/Game/Blueprints/Timeinfo` (`|GetArrayItem` _timeframes_2 _returnvalue_2)))
        (set `self.RecordTimeLength` (- (`self.RecordTimeLength`) _output_deltatime))
        (`KismetArrayLibrary.Array_Remove` (`self.TimeFrames`) _returnvalue_2))
      (else
        (`self.SetActorInfo` _timeframes)
        (`KismetArrayLibrary.Array_Clear` (`self.TimeFrames`))
        (set `self.RecordTimeLength` 0.0)
        (set `self.IsOutData` true)))))

(fn `RecordTimeinfo`
  (params (DeltaTime :type "Float (double-precision)"))
  (bind _owner (`self.Owner`))
  (bind _timeframes (`self.TimeFrames`))
  (bind _returnvalue (`Actor.GetComponentByClass` _owner "/Script/Engine.StaticMeshComponent"))
  (bind (_output_location _output_rotation _output_linearvelocity _output_angularvelocity _output_deltatime) (break `/Game/Blueprints/Timeinfo` (`|GetArrayItem` _timeframes)))
  (`/Engine/EditorBlueprintResources/StandardMacros.IsValid` _returnvalue
    (:`Is Valid`
      (if (<= (`self.RecordTimeLength`) 10.0)
        (bind _returnvalue_2 (`PrimitiveComponent.GetPhysicsLinearVelocity` _returnvalue "None"))
        (else
          (set `self.RecordTimeLength` (- (`self.RecordTimeLength`) _output_deltatime))
          (`KismetArrayLibrary.Array_Remove` _timeframes)))
      (`KismetArrayLibrary.Array_Add` (`self.TimeFrames`) (make `/Game/Blueprints/Timeinfo` (`Actor.K2_GetActorLocation` _owner) (`Actor.K2_GetActorRotation` _owner) _returnvalue_2 (`PrimitiveComponent.GetPhysicsAngularVelocityInDegrees` _returnvalue "None") DeltaTime))
      (set `self.RecordTimeLength` (+ (`self.RecordTimeLength`) DeltaTime))
      (set `self.IsOutData` false))))

(fn `SetActorInfo`
  (params (Array :type "Array of /Game/Blueprints/Timeinfo Structure") (Index :type Integer))
  (bind (_output_location _output_rotation _output_linearvelocity _output_angularvelocity) (break `/Game/Blueprints/Timeinfo` (`|GetArrayItem` Array Index)))
  (bind _owner (`self.Owner`))
  (bind _returnvalue (`Actor.GetComponentByClass` (`self.Owner`) "/Script/Engine.StaticMeshComponent"))
  (`Actor.K2_SetActorLocation` _owner _output_location false false)
  (`Actor.K2_SetActorRotation` _owner _output_rotation false)
  (`PrimitiveComponent.SetPhysicsLinearVelocity` _returnvalue _output_linearvelocity false "None")
  (`PrimitiveComponent.SetPhysicsAngularVelocityInDegrees` _returnvalue _output_angularvelocity false "None"))